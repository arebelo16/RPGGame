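; Melee attack gameplay ability that turns the avatar toward its combat target and plays a random tagged attack montage.
; When the montage's gameplay event fires, it finds live players in a small sphere at that tag's combat socket, excluding the avatar, and calls CauseDamage on each.
; It ends when the montage completes, is interrupted or is cancelled, or when no montages are available.
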(event `self.K2_ActivateAbility`
  (bind _returnvalue (`self.GetAvatarActorFromActorInfo`))
  (bind _returnvalue_2 (`self.GetAvatarActorFromActorInfo`))
  (bind _returnvalue_3 (message `EnemyInterface.GetCombatTarget` _returnvalue_2))
  (bind _ascombat_interface (cast `CombatInterface` _returnvalue_2))
  (`CombatInterface.UpdateFacingTarget` _ascombat_interface (`Actor.K2_GetActorLocation` _returnvalue_3))
  (bind _returnvalue_4 (message `CombatInterface.GetAttackMontages` (`self.GetAvatarActorFromActorInfo`)))
  (bind (_montage _montagetag) (`self.GetRandomMontage` _returnvalue_4))
  (`AbilityTask_PlayMontageAndWait.CreatePlayMontageAndWaitProxy` "None" _montage
    (:`then`
      (`AbilityTask_WaitGameplayEvent.WaitGameplayEvent` _montagetag null
        (:`EventReceived`
          (bind _returnvalue_5 (message `CombatInterface.GetCombatSocketLocation` _returnvalue _montagetag))
          (bind _outoverlappingactors (`AuraAbillitySystemLibrary.GetLivePlayersWithinRadius` _returnvalue (`|MakeArray` _returnvalue) 45.0 _returnvalue_5))
          (for _array_element _outoverlappingactors
            (`self.CauseDamage` _array_element)))))
    (:`OnCompleted`
      (`self.K2_EndAbility` :!label _label))
    (:`OnInterrupted`
      (goto _label))
    (:`OnCancelled`
      (goto _label))))

(fn `GetRandomMontage`
  (params (Array :type "Array of TaggedMontage Structure"))
  (returns (Montage :type "AnimMontage Object Reference") (MontageTag :type "GameplayTag Structure"))
  (bind _returnvalue (`KismetArrayLibrary.Array_Length` Array))
  (if (> _returnvalue 0)
    (bind _output_get (set `self.TaggedMontage` (`|GetArrayItem` Array (`KismetMathLibrary.RandomIntegerInRange` 0 (- _returnvalue 1)))))
    (bind (_montage _montagetag) (break `TaggedMontage` _output_get))
    (return _montage _montagetag)
    (else
      (`self.K2_EndAbility`))))