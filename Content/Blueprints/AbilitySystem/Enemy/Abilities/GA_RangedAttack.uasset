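; Enemy Gameplay Ability that performs a ranged attack by firing a projectile at the avatar's combat target.
; On activation it turns the avatar toward the target and plays a randomly picked tagged attack montage from the avatar.
; The montage's gameplay event tag triggers SpawnProjectile once from the matching socket tag, aimed at the target's location re-read at that moment.
; The graph never calls EndAbility.
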(event `self.K2_ActivateAbility`
  (bind _returnvalue (`self.GetAvatarActorFromActorInfo`))
  (bind _returnvalue_2 (message `EnemyInterface.GetCombatTarget` _returnvalue))
  (message `CombatInterface.UpdateFacingTarget` _returnvalue (`Actor.K2_GetActorLocation` _returnvalue_2))
  (bind _returnvalue_3 (message `CombatInterface.GetAttackMontages` (`self.GetAvatarActorFromActorInfo`)))
  (bind (_montage _montagetag _sockettag) (`self.GetRandomMontage` _returnvalue_3))
  (`AbilityTask_PlayMontageAndWait.CreatePlayMontageAndWaitProxy` "None" _montage 1.0 "None" false
    (:`then`
      (`AbilityTask_WaitGameplayEvent.WaitGameplayEvent` _montagetag null true
        (:`EventReceived`
          (bind _returnvalue_4 (message `EnemyInterface.GetCombatTarget` (`self.GetAvatarActorFromActorInfo`)))
          (`self.SpawnProjectile` (`Actor.K2_GetActorLocation` _returnvalue_4) _sockettag))))))

(fn `GetRandomMontage`
  (params (Array :type "Array of TaggedMontage Structure"))
  (returns (Montage :type "AnimMontage Object Reference") (MontageTag :type "GameplayTag Structure") (SocketTag :type "GameplayTag Structure") (ImpactSound :type "SoundBase Object Reference"))
  (bind _output_get (set `self.TaggedMontage` (`self.GetRandomTaggedMontageFromArray` Array)))
  (bind (_montage _montagetag _sockettag _impactsound) (break `TaggedMontage` _output_get))
  (return _montage _montagetag _sockettag _impactsound))