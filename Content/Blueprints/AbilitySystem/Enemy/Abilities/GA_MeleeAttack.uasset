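; Enemy melee Gameplay Ability that damages hostile live players struck by a randomly chosen attack montage.
; It turns the avatar toward its combat target, plays the montage and waits for that montage's tagged gameplay event.
; The event triggers a small sphere check at the montage's socket, damaging non-friends found.
; A hit fires the MeleeImpact gameplay cue and ends the ability; otherwise it ends with the montage.
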(event `self.K2_ActivateAbility`
  (bind _returnvalue (`self.GetOwningActorFromActorInfo`))
  (bind _returnvalue_2 (`self.GetAvatarActorFromActorInfo`))
  (bind _returnvalue_3 (`self.GetAvatarActorFromActorInfo`))
  (set `self.HasHitTarget` false)
  (bind _returnvalue_4 (message `EnemyInterface.GetCombatTarget` _returnvalue_3))
  (bind _ascombat_interface (cast `CombatInterface` _returnvalue_3))
  (`CombatInterface.UpdateFacingTarget` _ascombat_interface (`Actor.K2_GetActorLocation` _returnvalue_4))
  (bind _returnvalue_5 (message `CombatInterface.GetAttackMontages` (`self.GetAvatarActorFromActorInfo`)))
  (bind (_montage _montagetag _impactsound _sockettag) (`self.GetRandomMontage` _returnvalue_5))
  (set `self.ImpactSound` _impactsound)
  (set `self.Montage Tag` _montagetag)
  (set `self.Socket Tag` _sockettag)
  (`AbilityTask_PlayMontageAndWait.CreatePlayMontageAndWaitProxy` "None" _montage
    (:`then`
      (`AbilityTask_WaitGameplayEvent.WaitGameplayEvent` (`self.Montage Tag`) null
        (:`EventReceived`
          (bind _returnvalue_6 (message `CombatInterface.GetCombatSocketLocation` _returnvalue_2 (`self.Socket Tag`)))
          (bind _output_get (set `self.CombatSocketLocation` _returnvalue_6))
          (bind _outoverlappingactors (`AuraAbilitySystemLibrary.GetLivePlayersWithinRadius` _returnvalue_2 (`|MakeArray` _returnvalue_2) 45.0 _output_get))
          (for _array_element _outoverlappingactors
            (if (`AuraAbilitySystemLibrary.IsNotFriend` (`self.GetAvatarActorFromActorInfo`) _array_element)
              (`self.CauseDamage` _array_element)
              (set `self.HasHitTarget` true)
              (message `CombatInterface.GetBloodEffect` _array_element)))
          (if (`self.HasHitTarget`)
            (bind _returnvalue_7 (message `EnemyInterface.GetCombatTarget` _returnvalue))
            (set `self.CombatTarget` _returnvalue_7)
            (`self.K2_ExecuteGameplayCueWithParams` (struct :`TagName` "GameplayCue.MeleeImpact") (`AbilitySystemBlueprintLibrary.MakeGameplayCueParameters` 0.0 0.0 (struct) (struct) (struct) (`BlueprintGameplayTagLibrary.MakeGameplayTagContainerFromTag` (`.MontageTag` (break `TaggedMontage` (`self.TaggedMontage`)))) (struct) (`self.CombatSocketLocation`) (0.0 0.0 0.0) null _returnvalue (`self.CombatTarget`)))
            (`self.K2_EndAbility`)))))
    (:`OnCompleted`
      (`self.K2_EndAbility` :!label _label))
    (:`OnInterrupted`
      (goto _label))
    (:`OnCancelled`
      (goto _label))))

(fn `GetRandomMontage`
  (params (Array :type "Array of TaggedMontage Structure"))
  (returns (Montage :type "AnimMontage Object Reference") (MontageTag :type "GameplayTag Structure") (ImpactSound :type "SoundBase Object Reference") (SocketTag :type "GameplayTag Structure"))
  (bind _output_get (set `self.TaggedMontage` (`self.GetRandomTaggedMontageFromArray` Array)))
  (bind (_montage _montagetag _sockettag _impactsound) (break `TaggedMontage` _output_get))
  (return _montage _montagetag _impactsound _sockettag))